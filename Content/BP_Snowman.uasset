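; BP_Snowman is a snowman Blueprint with a simple procedural leg-swing animation that the Space Bar toggles on and off.
; While animating, Tick advances a Time value scaled by Speed and uses its sine to pitch the HipL and HipR components in opposite directions.
; Toggling off freezes the pose, since Time and the hip rotations are left as they are.
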(event `self.ReceiveTick`
  (params (DeltaSeconds :type "Float (single-precision)"))
  (if (`self.bAnimating`)
    (bind _output_get (set `self.Time` (+ (* DeltaSeconds (`self.Speed`)) (`self.Time`))))
    (bind _returnvalue (`KismetMathLibrary.Sin` _output_get))
    (`SceneComponent.K2_SetRelativeRotation` (`self.HipL`) (`KismetMathLibrary.MakeRotator` 0.0 (* _returnvalue 45.0)) false false)
    (`SceneComponent.K2_SetRelativeRotation` (`self.HipR`) (`KismetMathLibrary.MakeRotator` 0.0 (* _returnvalue -45.0)) false false)))

(event `Key|SpaceBar` :consume false
  (params (Key :type "Key Structure"))
  (:`Pressed`
    (set `self.bAnimating` (not (`self.bAnimating`)))))

(fn `UserConstructionScript`)